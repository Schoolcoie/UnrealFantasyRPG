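; Player controller for the Uriel character that turns player input into movement and crouching on the controlled pawn.
; MoveForward and MoveRight axes add movement input along the pawn's own forward and right vectors.
; The Crouch action casts the pawn to CBP_Uriel, crouching on press and uncrouching on release, so it works as hold-to-crouch.
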(event Input|ActionEvents|InputActionCrouch
  (params (Key :type Key%20Structure :default "None"))
  (bind _returnvalue (Pawn|GetControlledPawn))
  (:Pressed
    (bind _ascbp_uriel (Utilities|Casting|CastToCBP_Uriel _returnvalue))
    (Character|Crouch _ascbp_uriel))
  (:Released
    (bind _ascbp_uriel_2 (Utilities|Casting|CastToCBP_Uriel _returnvalue))
    (Character|UnCrouch _ascbp_uriel_2)))

(event Input|AxisEvents|InputAxisMoveRight
  (params (AxisValue :type Float%20%28single-precision%29))
  (bind _returnvalue (Pawn|GetControlledPawn))
  (Pawn|Input|AddMovementInput _returnvalue (Transformation|GetActorRightVector _returnvalue) AxisValue false))

(event Input|AxisEvents|InputAxisMoveForward
  (params (AxisValue :type Float%20%28single-precision%29))
  (bind _returnvalue (Pawn|GetControlledPawn))
  (Pawn|Input|AddMovementInput _returnvalue (Transformation|GetActorForwardVector _returnvalue) AxisValue false))

(fn ConstructionScript)